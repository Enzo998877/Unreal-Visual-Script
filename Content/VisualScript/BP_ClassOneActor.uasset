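; BP_ClassOneActor is a scripting exercise actor that demonstrates debug output, particle spawning and timed movement.
; On BeginPlay it prints two messages, draws a debug sphere and cylinder, and spawns a tutorial particle emitter at one hardcoded world point.
; A chain of Delays then offsets the emitter sideways, applies a zero offset to it, and finally moves the StaticMesh component in the opposite direction.
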(event EventBeginPlay
  (Development|PrintString "Hello" true true "(R=0.083333,G=0.000000,B=0.003508,A=1.000000)" 1e+01)
  (Development|PrintString "World" true true "(R=1.000000,G=0.802083,B=0.821157,A=1.000000)" 1e+01)
  (Rendering|Debug|DrawDebugSphere "560.000000,880.000000,0.000000" 1e+03 12 "(R=1.000000,G=1.000000,B=1.000000,A=1.000000)" 1e+01 1.0)
  (Class|KismetSystemLibrary|DrawDebugCylinder "560.000000,880.000000,0.000000" "560.000000,880.000000,200.000000" 1e+02 12 "(R=1.000000,G=0.746353,B=0.295584,A=1.000000)" 0.0 0.0)
  (bind _returnvalue (Effects|SpawnEmitteratLocation "/Engine/Tutorial/SubEditors/TutorialAssets/TutorialParticleSystem.TutorialParticleSystem" "560.000000,880.000000,0.000000"))
  (Utilities|FlowControl|Delay 3.0)
  (Transformation|AddWorldOffset _returnvalue "0.000000,200.000000,0.000000" false false)
  (Utilities|FlowControl|Delay 3.0)
  (Transformation|AddWorldOffset _returnvalue "0, 0, 0" false false)
  (Utilities|FlowControl|Delay 3.0)
  (Transformation|AddWorldOffset (Variables|Default|GetStaticMesh) "0.000000,-200.000000,0.000000" false false))

(fn ConstructionScript)